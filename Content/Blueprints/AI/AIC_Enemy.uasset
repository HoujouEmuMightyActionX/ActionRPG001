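; AIC_Enemy is the AI controller for robot enemies, running the enemy behavior tree and blackboard.
; On possess it binds to the robot's damaged-state switch and mirrors that state into the blackboard.
; SetAttackTarget stores the target in the blackboard.
; Each tick it aims focus toward the RPG character target along world X only while the robot can act, otherwise holding its current forward direction.
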(event Custom|OnDamagedStateChange
  (params (InDamagedState :type Boolean))
  (AI|Components|Blackboard|SetValueasBool (Variables|Default|GetBlackboard) (Utilities|Name|MakeLiteralName "DamagedState") InDamagedState))

(event EventBeginPlay
  (Class|AIController|UseBlackboard "/Game/Blueprints/AI/BB_Enemy.BB_Enemy")
  (AI|RunBehaviorTree "/Game/Blueprints/AI/BT_Enemy.BT_Enemy"))

(event EventTick
  (params (DeltaSeconds :type Float%20%28single-precision%29))
  (CallFunction|SetFocusDirection))

(event EventPossess
  (params (PossessedPawn :type Pawn%20Object%20Reference))
  (bind _asbp_robot (Utilities|Casting|CastToBP_Robot PossessedPawn))
  (bind _output_get (Variables|Default|SetRobot _asbp_robot))
  (EventDispatchers|BindEventtoDamagedStateSwitch _output_get (delegate Custom|OnDamagedStateChange)))

(fn ConstructionScript)

(fn SetAttackTarget
  (params (AttackTarget :type BP%20Yusuke%20Object%20Reference))
  (AI|Components|Blackboard|SetValueasObject (Variables|Default|GetBlackboard) (Variables|Default|GetAttackTargetKey) AttackTarget)
  (Variables|Default|SetAttack%20Target AttackTarget))

(fn SetFocusDirection
  (Utilities|IsValid (AI|Components|Blackboard|GetValueasObject (Variables|Default|GetBlackboard) (Variables|Default|GetAttackTargetKey))
    (:Is%20Valid
      (if (Default|CanActCheck (Variables|Default|GetRobot))
        (bind _asbp_rpgchar (Utilities|Casting|CastToBP_RPGChar (AI|Components|Blackboard|GetValueasObject (Variables|Default|GetBlackboard) (Variables|Default|GetAttackTargetKey))))
        (AI|SetFocalPoint (+ (Transformation|GetActorLocation (Variables|Default|GetRobot)) (Math|Vector|MakeVector (.x (Math|Vector|GetForwardVector (Math|Rotator|FindLookatRotation (Transformation|GetActorLocation (Variables|Default|GetRobot)) (Transformation|GetActorLocation _asbp_rpgchar)))) 0.0 0.0)))
        (else
          (AI|SetFocalPoint (+ (Transformation|GetActorLocation (Variables|Default|GetRobot)) (Transformation|GetActorForwardVector (Variables|Default|GetRobot))) :!label _label))))
    (:Is%20Not%20Valid
      (goto _label))))