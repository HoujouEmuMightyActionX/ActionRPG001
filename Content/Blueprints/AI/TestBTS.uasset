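; Behavior tree service that flags whether BP_Enemy allies are near the controlled pawn along the Y axis.
; Each tick it runs a box overlap at the pawn's location, narrow in world X and long in Y, filtered to BP_Enemy and ignoring Player.
; It writes the result to the AlliesInY blackboard bool and prints that value for debugging.
; The pawn itself is not in the ignore list.
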(event EventReceiveTickAI
  (params (OwnerController :type AI%20Controller%20Object%20Reference) (ControlledPawn :type Pawn%20Object%20Reference) (DeltaSeconds :type Float%20%28single-precision%29))
  (bind _blackboard (Variables|/Script/AIModule.AIController|GetBlackboard OwnerController))
  (Variables|Default|SetRobot ControlledPawn)
  (bind _returnvalue (Collision|BoxOverlapActors (Transformation|GetActorLocation (Variables|Default|GetRobot)) "10.000000,200.000000,32.000000" (Variables|Default|GetObjectTypes) "/Game/Blueprints/Characters/Enemy/BP_Enemy.BP_Enemy_C" (Utilities|Array|MakeArray (Variables|Default|GetPlayer)) :!class /Script/Engine.KismetSystemLibrary))
  (AI|Components|Blackboard|SetValueasBool _blackboard (Utilities|Name|MakeLiteralName "AlliesInY") _returnvalue)
  (Development|PrintString (Utilities|String|Append "alliesinY" (Utilities|String|ToString(Boolean) (ScalableFloat|GetValueasBool _blackboard (Utilities|Name|MakeLiteralName "AlliesInY"))))))