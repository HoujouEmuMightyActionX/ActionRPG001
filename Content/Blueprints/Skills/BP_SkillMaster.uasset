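; BP_SkillMaster is a skill actor, apparently a base for specific skills, that performs an attack on BP_RPGChar.
; ActivateAttack finds the character via GetActorOfClass, flags it as attacking and plays the skill's animation as an override in the Attack slot.
; As playback starts, SkillInfo sets the character's hitbox size and position, attack type and stage.
; The attacking flag clears only when the animation's Completed callback fires.
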(event Custom|ActivateAttack
  (bind _skillinfo (Variables|Default|GetSkillInfo))
  (bind (_atktype _damage _airborne _hitboxextent _hitboxpos _attackstage) (Utilities|Struct|BreakF_Skills _skillinfo))
  (bind _returnvalue (Actor|GetActorOfClass "/Game/Blueprints/Characters/BP_RPGChar.BP_RPGChar_C"))
  (Variables|Default|SetAttacker _returnvalue)
  (Variables|/Game/Blueprints/Characters/BP_RPGChar.BP_RPGChar_C|SetIsAttacking (Variables|Default|GetAttacker) true)
  (|PlayAnimationOverridewithCallbacks (Class|PaperZDCharacter|GetAnimInstance (Variables|Default|GetAttacker)) (Variables|Default|GetAnim%20Sequence) "Attack" 1.0 0.0
    (:then
      (CallFunction|SetHitboxExtentPos (Variables|Default|GetAttacker))
      (Variables|/Game/Blueprints/Characters/BP_RPGChar.BP_RPGChar_C|SetCurrentAtkType (Variables|Default|GetAttacker) _atktype)
      (Variables|/Game/Blueprints/Characters/Yusuke/BP_Yusuke.BP_Yusuke_C|SetAttackStage (Variables|Default|GetAttacker) _attackstage))
    (:OnCompleted
      (Variables|/Game/Blueprints/Characters/BP_RPGChar.BP_RPGChar_C|SetIsAttacking (Variables|Default|GetAttacker) false))))

(event EventBeginPlay)

(event Collision|EventActorBeginOverlap
  (params (OtherActor :type Actor%20Object%20Reference)))

(event EventTick
  (params (DeltaSeconds :type Float%20%28single-precision%29)))

(fn ConstructionScript)

(fn SetHitboxExtentPos
  (params (Attacker :type BP%20RPG%20Char%20Object%20Reference%20%28by%20ref%29))
  (bind _skillinfo (Variables|Default|GetSkillInfo))
  (bind (_atktype _damage _airborne _hitboxextent _hitboxpos) (Utilities|Struct|BreakF_Skills _skillinfo))
  (Components|Box|SetBoxExtent (Variables|/Game/Blueprints/Characters/BP_RPGChar.BP_RPGChar_C|GetHitbox Attacker) _hitboxextent true)
  (Transformation|SetRelativeLocation (Variables|/Game/Blueprints/Characters/BP_RPGChar.BP_RPGChar_C|GetHitbox Attacker) _hitboxpos false false))