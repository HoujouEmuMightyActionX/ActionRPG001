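; TestCamera is a side-on spring-arm camera that frames the player character and their current AttackTarget.
; Each Tick, it derives arm length from a sine of their clamped X separation, downward pitch from that separation squared, and a clamped target offset from both positions.
; BlendScopeTarget suspends that update while the ScopeBlend timeline lerps the arm toward similarly computed framing, then hands control back to Tick.
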(event EventBeginPlay
  (bind _asbp_rpgchar (Utilities|Casting|CastToBP_RPGChar (Game|GetPlayerCharacter 0)))
  (bind _output_get (Variables|Default|SetPlayer _asbp_rpgchar))
  (Variables|Default|SetScopeTarget (Variables|/Game/Blueprints/Characters/BP_RPGChar.BP_RPGChar_C|GetAttackTarget _output_get)))

(event Collision|EventActorBeginOverlap
  (params (OtherActor :type Actor%20Object%20Reference)))

(event EventTick
  (params (DeltaSeconds :type Float%20%28single-precision%29))
  (bind _player (Variables|Default|GetPlayer))
  (bind _player_2 (Variables|Default|GetPlayer))
  (bind _springarm (Variables|Default|GetSpringArm))
  (bind _returnvalue (Transformation|GetWorldLocation _springarm))
  (bind _returnvalue_2 (Transformation|GetActorLocation _player))
  (bind _attacktarget (Variables|/Game/Blueprints/Characters/BP_RPGChar.BP_RPGChar_C|GetAttackTarget _player_2))
  (bind _returnvalue_3 (Transformation|GetActorLocation _attacktarget))
  (bind _returnvalue_4 (- (.x _returnvalue_3) (.x _returnvalue_2)))
  (bind _returnvalue_5 (Math|Float|Absolute(Float) _returnvalue_4))
  (if (not (Variables|Default|GetCameraIsBlending))
    (Variables|/Script/Engine.SpringArmComponent|SetTargetArmLength (Variables|Default|GetSpringArm) (+ (* (Math|Trig|Sin(Radians) (/ (- (Math|Float|Clamp(Float) _returnvalue_5 4.6e+02 1.6e+03) 4e+02) 6.2e+02)) 2.8e+03) 1.4e+03))
    (Transformation|SetRelativeRotation (Variables|Default|GetSpringArm) (Math|Rotator|MakeRotator 0.0 (Math|Float|Clamp(Float) (/ (Math|Float|Power (/ _returnvalue_5 1e+02) 2.0) -1e+01) -2e+01 0.0) -9e+01) false false)
    (Variables|/Script/Engine.SpringArmComponent|SetTargetOffset (Variables|Default|GetSpringArm) (Math|Vector|MakeVector (Math|Float|Clamp(Float) (/ (+ (- (.x _returnvalue_3) (.x _returnvalue)) (- (.x _returnvalue_2) (.x _returnvalue))) 2.0) -8e+02 8e+02) (.y (Transformation|GetActorLocation (Variables|Default|GetPlayer))) (Math|Float|Clamp(Float) (/ (+ (- (.z _returnvalue_3) (.y _returnvalue)) (- (.z _returnvalue_2) (.z _returnvalue))) 2.0) 3e+01 5e+02)))))

(event EventBlendScopeTarget
  (bind _player (Variables|Default|GetPlayer))
  (bind _springarm (Variables|Default|GetSpringArm))
  (bind _player_2 (Variables|Default|GetPlayer))
  (bind _returnvalue (Transformation|GetActorLocation _player_2))
  (bind _returnvalue_2 (Transformation|GetWorldLocation _springarm))
  (bind _attacktarget (Variables|/Game/Blueprints/Characters/BP_RPGChar.BP_RPGChar_C|GetAttackTarget _player))
  (bind _returnvalue_3 (Transformation|GetActorLocation _attacktarget))
  (bind _returnvalue_4 (- (.x _returnvalue_3) (.x _returnvalue)))
  (bind _returnvalue_5 (Math|Float|Absolute(Float) _returnvalue_4))
  (Variables|Default|SetCameraIsBlending true)
  (Components|Timeline|SetPlayRate (Variables|Default|GetScopeBlend) 1.2)
  (bind _scopeblend (Timeline|ScopeBlend PlayFromStart)
    (:Update
      (Variables|/Script/Engine.SpringArmComponent|SetTargetArmLength (Variables|Default|GetSpringArm) (Math|Float|Lerp (Variables|/Script/Engine.SpringArmComponent|GetTargetArmLength (Variables|Default|GetSpringArm)) (+ (* (Math|Trig|Sin(Radians) (/ (- (Math|Float|Clamp(Float) _returnvalue_5 4.6e+02 1.6e+03) 4e+02) 6.2e+02)) 2.8e+03) 1.4e+03) _scopeblend))
      (Transformation|SetRelativeRotation (Variables|Default|GetSpringArm) (Math|Rotator|MakeRotator 0.0 (Math|Float|Lerp (.pitch (Variables|/Script/Engine.SceneComponent|GetRelativeRotation (Variables|Default|GetSpringArm))) (Math|Float|Clamp(Float) (/ (Math|Float|Power (/ _returnvalue_5 1e+02) 2.0) -1e+01) -2e+01 0.0) _scopeblend) -9e+01) false false)
      (Variables|/Script/Engine.SpringArmComponent|SetTargetOffset (Variables|Default|GetSpringArm) (Math|Vector|Lerp(Vector) (Variables|/Script/Engine.SpringArmComponent|GetTargetOffset (Variables|Default|GetSpringArm)) (Math|Vector|MakeVector (Math|Float|Clamp(Float) (/ (+ (- (.x _returnvalue_3) (.x _returnvalue_2)) (- (.x _returnvalue) (.x _returnvalue_2))) 2.0) -8e+02 8e+02) (.y (Transformation|GetActorLocation (Variables|Default|GetPlayer))) (Math|Float|Clamp(Float) (/ (+ (- (.z _returnvalue_3) (.z _returnvalue_2)) (- (.z _returnvalue) (.z _returnvalue_2))) 2.0) 3e+01 5e+02)) _scopeblend)))
    (:Finished
      (Variables|Default|SetCameraIsBlending false))))

(fn ConstructionScript)