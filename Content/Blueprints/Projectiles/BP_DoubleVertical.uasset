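; BP_DoubleVertical is a projectile with two collision spheres that each apply damage to any BP_Enemy they begin overlapping.
; Only the first sphere ends its life, destroying the actor shortly after a blocking hit or when it stops overlapping an enemy.
; A HitStopSequence event, not called within this graph, briefly freezes the projectile through CustomTimeDilation using retriggerable start and length delays.
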(event OnComponentHit(Sphere)
  (params (HitComponent :type Primitive%20Component%20Object%20Reference) (OtherActor :type Actor%20Object%20Reference) (OtherComp :type Primitive%20Component%20Object%20Reference) (NormalImpulse :type Vector :default "0, 0, 0") (Hit :type Hit%20Result%20Structure%20%28by%20ref%29))
  (if (.bBlockingHit (Collision|BreakHitResult Hit))
    (Utilities|FlowControl|Delay 0.1)
    (Actor|DestroyActor)))

(event OnComponentBeginOverlap(Sphere)
  (params (OverlappedComponent :type Primitive%20Component%20Object%20Reference) (OtherActor :type Actor%20Object%20Reference) (OtherComp :type Primitive%20Component%20Object%20Reference) (OtherBodyIndex :type Integer) (bFromSweep :type Boolean) (SweepResult :type Hit%20Result%20Structure%20%28by%20ref%29))
  (bind _asbp_enemy (Utilities|Casting|CastToBP_Enemy OtherActor))
  (Game|Damage|ApplyDamage _asbp_enemy 1e+01 0 self "/Script/Engine.DamageType"))

(event OnComponentEndOverlap(Sphere)
  (params (OverlappedComponent :type Primitive%20Component%20Object%20Reference) (OtherActor :type Actor%20Object%20Reference) (OtherComp :type Primitive%20Component%20Object%20Reference) (OtherBodyIndex :type Integer))
  (Utilities|Casting|CastToBP_Enemy OtherActor)
  (Actor|DestroyActor))

(event OnComponentBeginOverlap(Sphere2)
  (params (OverlappedComponent :type Primitive%20Component%20Object%20Reference) (OtherActor :type Actor%20Object%20Reference) (OtherComp :type Primitive%20Component%20Object%20Reference) (OtherBodyIndex :type Integer) (bFromSweep :type Boolean) (SweepResult :type Hit%20Result%20Structure%20%28by%20ref%29))
  (bind _asbp_enemy (Utilities|Casting|CastToBP_Enemy OtherActor))
  (Game|Damage|ApplyDamage _asbp_enemy 1e+01 0 self "/Script/Engine.DamageType"))

(event Custom|HitStopSequence
  (params (HitStopStartDelay :type Float%20%28single-precision%29) (HitStoplength :type Float%20%28single-precision%29))
  (Utilities|FlowControl|RetriggerableDelay HitStopStartDelay)
  (Variables|Default|SetCustomTimeDilation 0.0)
  (Utilities|FlowControl|RetriggerableDelay HitStoplength)
  (Variables|Default|SetCustomTimeDilation 1.0))

(event EventBeginPlay)

(event Collision|EventActorBeginOverlap
  (params (OtherActor :type Actor%20Object%20Reference)))

(event EventTick
  (params (DeltaSeconds :type Float%20%28single-precision%29)))

(fn ConstructionScript)