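; Player-controlled character Blueprint for Yusuke in a side-facing action RPG battle, handling movement, combos, specials, guard and evade.
; Enhanced Input plus sensed stick direction selects attack and special requests sent to the AnimInstance.
; Charge time picks SP2's projectile and knockback; SP4 vanishes, box-traces, then teleports or dashes to smash.
; It also tracks enemy targets and a Chain Capacity resource, spent on attacks and regained over time or by evading hits, updating the HUD.
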(event OnComponentBeginOverlap(Hitbox)
  (params (OverlappedComponent :type Primitive%20Component%20Object%20Reference) (OtherActor :type Actor%20Object%20Reference) (OtherComp :type Primitive%20Component%20Object%20Reference) (OtherBodyIndex :type Integer) (bFromSweep :type Boolean) (SweepResult :type Hit%20Result%20Structure%20%28by%20ref%29))
  (if (>= (Variables|Default|GetCriticalCage) 0.99)
    (CallFunction|AddCC 1)))

(event Custom|Evade
  (Utilities|FlowControl|DoOnce false :!label _label
    (:Completed
      (Class|BPICombo|RequestEvade(Message) (Variables|/Script/PaperZD.PaperZDAnimationComponent|GetAnimInstance (Variables|Default|GetAnimationComponent)) (Variables|Default|GetDirectionalInput))
      (Variables|Default|SetIsGuarding false)
      (Variables|Default|SetIsEvading true)
      (Variables|Default|SetDamageReduceRate 0.0)
      (Variables|AttackParameter|SetEvadeStartLocation (Transformation|GetActorLocation))
      (bind _returnvalue (CallFunction|SetEvadeVector))
      (Components|Timeline|SetPlayRate (Variables|Default|GetEvadeTimeline) 1e+01)
      (bind _evadecurve (Timeline|EvadeTimeline PlayFromStart)
        (:Update
          (Transformation|SetActorRelativeLocation (Math|Vector|Lerp(Vector) (Variables|AttackParameter|GetEvadeStartLocation) _returnvalue _evadecurve) true)
          (Utilities|FlowControl|RetriggerableDelay 0.01)
          (goto _label Reset))
        (:Finished
          (Variables|Default|SetIsEvading false))))))

(event Custom|ResetComboHits)

(event Input|EnhancedActionEvents|EnhancedInputActionIA_Special
  (params (ActionValue :type Boolean) (ElapsedSeconds :type Float%20%28double-precision%29) (TriggeredSeconds :type Float%20%28double-precision%29) (InputAction :type Input%20Action%20Object%20Reference :default "/Game/Inputs/Actions/IA_Special.IA_Special"))
  (:Started
    (if (CallFunction|CanActCheck)
      (bind _requestedattack (CallFunction|SetAttackDirection))
      (switch Utilities|FlowControl|Switch|SwitchonE_ComboInputs _requestedattack
        (:NewEnumerator0
          (Class|BPICombo|RequestSP(Message) (Variables|/Script/PaperZD.PaperZDAnimationComponent|GetAnimInstance (Variables|Default|GetAnimationComponent)) "NewEnumerator0"))
        (:NewEnumerator1
          (Class|BPICombo|RequestSP(Message) (Variables|/Script/PaperZD.PaperZDAnimationComponent|GetAnimInstance (Variables|Default|GetAnimationComponent)) "NewEnumerator5"))
        (:NewEnumerator3
          (Class|BPICombo|RequestSP(Message) (Variables|/Script/PaperZD.PaperZDAnimationComponent|GetAnimInstance (Variables|Default|GetAnimationComponent)) "NewEnumerator7"))
        (:NewEnumerator4
          (Class|BPICombo|RequestSP(Message) (Variables|/Script/PaperZD.PaperZDAnimationComponent|GetAnimInstance (Variables|Default|GetAnimationComponent)) "NewEnumerator3"))))))

(event Input|EnhancedActionEvents|EnhancedInputActionIA_Move
  (params (ActionValue :type Vector%202D%20Structure) (ElapsedSeconds :type Float%20%28double-precision%29) (TriggeredSeconds :type Float%20%28double-precision%29) (InputAction :type Input%20Action%20Object%20Reference :default "/Game/Inputs/Actions/IA_Move.IA_Move"))
  (bind (_x _y) (Math|Vector2D|BreakVector2D ActionValue))
  (if (CallFunction|CanActCheck)
    (if (not (Variables|Default|GetCanNotMove))
      (Pawn|Input|AddMovementInput "1.000000,0.000000,0.000000" _x false)
      (Pawn|Input|AddMovementInput "0.000000,-1.000000,0.000000" (* _y 0.8) false))))

(event Input|EnhancedActionEvents|EnhancedInputActionIA_Jump
  (params (ActionValue :type Boolean) (ElapsedSeconds :type Float%20%28double-precision%29) (TriggeredSeconds :type Float%20%28double-precision%29) (InputAction :type Input%20Action%20Object%20Reference :default "/Game/Inputs/Actions/IA_Jump.IA_Jump"))
  (:Started
    (if (Variables|Default|GetIsGuarding)
      (Default|CallPressJumpWhileGuardtoEvade)
      (elif (and (CallFunction|CanJumpCheck) (CallFunction|CanActCheck))
        (Character|Jump))))
  (:Completed
    (Character|StopJumping)))

(event Input|EnhancedActionEvents|EnhancedInputActionIA_Special2
  (params (ActionValue :type Boolean) (ElapsedSeconds :type Float%20%28double-precision%29) (TriggeredSeconds :type Float%20%28double-precision%29) (InputAction :type Input%20Action%20Object%20Reference :default "/Game/Inputs/Actions/IA_Special2.IA_Special2"))
  (:Started
    (if (CallFunction|CanActCheck)
      (Class|BPICombo|RequestSP2ChargeStart(Message) (Variables|/Script/PaperZD.PaperZDAnimationComponent|GetAnimInstance (Variables|Default|GetAnimationComponent)) 0.0)))
  (:Completed
    (if (CallFunction|CanActCheck)
      (Class|BPICombo|RequestSP2Shoot(Message) (Variables|/Script/PaperZD.PaperZDAnimationComponent|GetAnimInstance (Variables|Default|GetAnimationComponent)))
      (Variables|AttackParameter|SetSP2ChargeTime TriggeredSeconds))))

(event Input|EnhancedActionEvents|EnhancedInputActionIA_NeutralAttack
  (params (ActionValue :type Boolean) (ElapsedSeconds :type Float%20%28double-precision%29) (TriggeredSeconds :type Float%20%28double-precision%29) (InputAction :type Input%20Action%20Object%20Reference :default "/Game/Inputs/Actions/IA_NeutralAttack.IA_NeutralAttack"))
  (bind _animationcomponent (Variables|Default|GetAnimationComponent))
  (bind _animinstance (Variables|/Script/PaperZD.PaperZDAnimationComponent|GetAnimInstance _animationcomponent))
  (:Started
    (if (CallFunction|CanActCheck)
      (if (AI|Components|NavMovement|IsFalling (Variables|Character|GetCharacterMovement))
        (Class|BPICombo|RequestCombo(Message) _animinstance "NewEnumerator5")
        (else
          (bind _requestedattack (CallFunction|SetAttackDirection))
          (Class|BPICombo|RequestCombo(Message) _animinstance _requestedattack))))))

(event Input|EnhancedActionEvents|EnhancedInputActionIA_Guard
  (params (ActionValue :type Boolean) (ElapsedSeconds :type Float%20%28double-precision%29) (TriggeredSeconds :type Float%20%28double-precision%29) (InputAction :type Input%20Action%20Object%20Reference :default "/Game/Inputs/Actions/IA_Guard.IA_Guard"))
  (:Triggered
    (Variables|Default|SetIsGuarding true)
    (Variables|Default|SetDamageReduceRate 0.5)
    (EventDispatchers|BindEventtoPressJumpWhileGuardtoEvade (delegate Custom|Evade)))
  (:Completed
    (Variables|Default|SetIsGuarding false)
    (Variables|Default|SetDamageReduceRate 0.0)))

(event Input|EnhancedActionEvents|EnhancedInputActionIA_Test
  (params (ActionValue :type Boolean) (ElapsedSeconds :type Float%20%28double-precision%29) (TriggeredSeconds :type Float%20%28double-precision%29) (InputAction :type Input%20Action%20Object%20Reference :default "/Game/Inputs/Actions/IA_Test.IA_Test"))
  (:Started
    (bind _returnvalue (Actor|GetActorOfClass "/Game/Blueprints/TestCamera.TestCamera_C"))
    (bind _outactors (Actor|GetAllActorsOfClass "/Game/Blueprints/Characters/Enemy/Robot/BP_Robot.BP_Robot_C"))
    (bind _array_element (Utilities|Array|ForEachLoopwithBreak _outactors :!label _label)
      (:LoopBody
        (if (!= _array_element (Variables|Default|GetAttackTarget))
          (Variables|Default|SetAttackTarget _array_element)
          (goto _label Break)))
      (:Completed
        (Default|BlendScopeTarget _returnvalue)))))

(event EventBeginPlay
  (|CallParentFunction)
  (bind _as玩家控制器 (Utilities|Casting|CastToPlayerController (Pawn|GetController)))
  (Input|AddMappingContext (PlayerController|LocalPlayerSubsystems|GetEnhancedInputLocalPlayerSubsystem _as玩家控制器) "/Game/Inputs/IMC_ActionRPG.IMC_ActionRPG" 0 "(bIgnoreAllPressedKeysUntilRelease=True,bForceImmediately=False,bNotifyUserSettings=False)")
  (bind _returnvalue (UserInterface|CreateWidget "/Game/UI/WB_HUDBattle.WB_HUDBattle_C"))
  (UserInterface|Viewport|AddtoViewport _returnvalue 0)
  (Variables|Default|SetHUDReference _returnvalue)
  (CallFunction|GetAllEnemies)
  (CallFunction|SetFirstTarget))

(event Collision|EventActorBeginOverlap
  (params (OtherActor :type Actor%20Object%20Reference))
  (|CallParentFunction OtherActor) ; 此节点被禁用，将不会被调用。\n从引脚连出引线来编译功能。
)

(event EventRegainCC
  (if (< (Variables|Default|GetCurrentChainCapacity) (Variables|Default|GetStartChainCapacity)) :!label _label
    (Utilities|FlowControl|RetriggerableDelay (/ (Variables|Default|GetCCRegainCycle) (Math|Float|Power (Math|Conversions|ToFloat(Integer) (Variables|Default|GetCurrentChainCapacity)) 2.0)))
    (Variables|Default|SetCurrentChainCapacity (Math|Integer|Clamp(Integer) (+ (Variables|Default|GetCurrentChainCapacity) 1) 0 (Variables|Default|GetMaxChainCapacity)))
    (Default|UpdateCurrentCC (Variables|Default|GetHUDReference))
    (goto _label)))

(event EventBackwardAttack
  (bind _returnvalue (Pawn|GetController))
  (bind _returnvalue_2 (Pawn|GetController))
  (switch Utilities|FlowControl|Switch|SwitchonE_CharacterRotation (Variables|Default|GetCharacterRotation)
    (:NewEnumerator0
      (Utilities|IsValid _returnvalue_2
        (:Is%20Valid
          (Pawn|SetControlRotation _returnvalue_2 (Math|Rotator|MakeRotator 0.0 0.0 1.8e+02)))))
    (:NewEnumerator1
      (Utilities|IsValid _returnvalue
        (:Is%20Valid
          (Pawn|SetControlRotation _returnvalue (Math|Rotator|MakeRotator 0.0 0.0 0.0)))))))

(event EventTick
  (params (DeltaSeconds :type Float%20%28single-precision%29))
  (|CallParentFunction DeltaSeconds)
  (CallFunction|UpdateControllerRotation)
  (CallFunction|SenseDirectionalInput))

(event EventSP2Charging
  (params (SP2StateBack :type E_SP2State%20Enum :default "NewEnumerator0"))
  (Variables|AttackParameter|SetSP2State SP2StateBack))

(event EventSP2Shoot
  (Variables|AttackParameter|SetSP2State "NewEnumerator2")
  (Variables|AttackParameter|SetShootingLocation (Transformation|GetWorldLocation (Variables|Default|GetSprite)))
  (Utilities|FlowControl|RetriggerableDelay 0.16)
  (if (AI|Components|NavMovement|IsFalling (Variables|Character|GetCharacterMovement))
    (if (>= (Variables|AttackParameter|GetSP2ChargeTime) 1.2)
      (Game|SpawnActorfromClass "/Game/Blueprints/Projectiles/BP_SP2AirBig.BP_SP2AirBig_C" (Math|Transform|MakeTransform (Transformation|GetWorldLocation (Variables|Default|GetSP2FullAirShootPos)) (Transformation|GetActorRotation) "1.000000,1.000000,1.000000") "AlwaysSpawn" "MultiplyWithRoot" 0 0)
      (Components|Timeline|SetPlayRate (Variables|Default|GetShootKnockback) 2e+01)
      (bind _airshootknockback (Timeline|ShootKnockback PlayFromStart)
        (:Update
          (if (Utilities|Enum|Equal(Enum) (Variables|Default|GetCharacterRotation) "NewEnumerator0")
            (Transformation|SetWorldLocation (Variables|Default|GetCapsuleComponent) (Math|Vector|Lerp(Vector) (Variables|AttackParameter|GetShootingLocation) (+ (Variables|AttackParameter|GetShootingLocation) "-10.000000,0.000000,10.000000") _airshootknockback) false false)
            (Variables|/Script/Engine.MovementComponent|SetVelocity (Variables|Character|GetCharacterMovement) "0, 0, 0")
            (else
              (Transformation|SetWorldLocation (Variables|Default|GetCapsuleComponent) (Math|Vector|Lerp(Vector) (Variables|AttackParameter|GetShootingLocation) (+ (Variables|AttackParameter|GetShootingLocation) "10.000000,0.000000,10.000000") _airshootknockback) false false)
              (Variables|/Script/Engine.MovementComponent|SetVelocity (Variables|Character|GetCharacterMovement) "0, 0, 0")))))
      (elif (>= (Variables|AttackParameter|GetSP2ChargeTime) 0.4)
        (Game|SpawnActorfromClass "/Game/Blueprints/Projectiles/BP_DoubleDown.BP_DoubleDown_C" (Math|Transform|MakeTransform (Transformation|GetWorldLocation (Variables|Default|GetSP2InstantShootAirPos)) (Transformation|GetActorRotation) "1.000000,1.000000,1.000000") "AlwaysSpawn" "MultiplyWithRoot" 0 0)
        (else
          (Game|SpawnActorfromClass "/Game/Blueprints/Projectiles/BP_SmallDown.BP_SmallDown_C" (Math|Transform|MakeTransform (Transformation|GetWorldLocation (Variables|Default|GetSP2InstantShootAirPos)) (Transformation|GetActorRotation) "1.000000,1.000000,1.000000") "AlwaysSpawn" "MultiplyWithRoot" 0 0))))
    (elif (>= (Variables|AttackParameter|GetSP2ChargeTime) 1.2)
      (Game|SpawnActorfromClass "/Game/Blueprints/Projectiles/BP_SP2GroundBig.BP_SP2GroundBig_C" (Math|Transform|MakeTransform (Transformation|GetWorldLocation (Variables|Default|GetSP2FullGroundShootPos)) (Transformation|GetActorRotation) "1.000000,1.000000,1.000000") "AlwaysSpawn" "MultiplyWithRoot" 0 0)
      (Components|Timeline|SetPlayRate (Variables|Default|GetShootKnockbackGround) 12.0)
      (bind _airshootknockback_2 (Timeline|ShootKnockbackGround PlayFromStart)
        (:Update
          (if (Utilities|Enum|Equal(Enum) (Variables|Default|GetCharacterRotation) "NewEnumerator0")
            (Transformation|SetWorldLocation (Variables|Default|GetCapsuleComponent) (Math|Vector|Lerp(Vector) (Variables|AttackParameter|GetShootingLocation) (+ (Variables|AttackParameter|GetShootingLocation) "-100.000000,0.000000,0.000000") _airshootknockback_2) false false)
            (else
              (Transformation|SetWorldLocation (Variables|Default|GetCapsuleComponent) (Math|Vector|Lerp(Vector) (Variables|AttackParameter|GetShootingLocation) (+ (Variables|AttackParameter|GetShootingLocation) "100.000000,0.000000,0.000000") _airshootknockback_2) false false)))))
      (elif (>= (Variables|AttackParameter|GetSP2ChargeTime) 0.4)
        (Game|SpawnActorfromClass "/Game/Blueprints/Projectiles/BP_DoubleVertical.BP_DoubleVertical_C" (Math|Transform|MakeTransform (Transformation|GetWorldLocation (Variables|Default|GetSP2InstantShootPos)) (Transformation|GetActorRotation) "1.000000,1.000000,1.000000") "AlwaysSpawn" "MultiplyWithRoot" 0 0)
        (else
          (Game|SpawnActorfromClass "/Game/Blueprints/Projectiles/BP_SmallVertical.BP_SmallVertical_C" (Math|Transform|MakeTransform (Transformation|GetWorldLocation (Variables|Default|GetSP2InstantShootPos)) (Transformation|GetActorRotation) "1.000000,1.000000,1.000000") "AlwaysSpawn" "MultiplyWithRoot" 0 0))))))

(event EventSP4Mechanics
  (Variables|Default|SetSP4StartLocation (Transformation|GetActorLocation))
  (Variables|/Script/Engine.CharacterMovementComponent|SetGravityScale (Variables|Character|GetCharacterMovement) 0.0)
  (Utilities|FlowControl|RetriggerableDelay 0.1)
  (Rendering|SetVisibility (Variables|Default|GetSprite) false false)
  (bind _outactors (Actor|GetAllActorsOfClass "/Game/Blueprints/Characters/NPC/BP_NPC.BP_NPC_C"))
  (Collision|SetCollisionResponsetoChannel (Variables|Default|GetCapsuleComponent) "ECC_Pawn" "ECR_Ignore")
  (Utilities|FlowControl|RetriggerableDelay 0.6)
  (Collision|SetCollisionResponsetoChannel (Variables|Default|GetCapsuleComponent) "ECC_Pawn" "ECR_Overlap")
  (bind (_outhit _returnvalue) (Class|KismetSystemLibrary|BoxTraceSingleforObjects (Variables|Default|GetSP4StartLocation) (+ (Variables|Default|GetSP4StartLocation) (* (Variables|Default|GetSP4TraceDistance) (Math|Vector|GetForwardVector (Variables|Default|GetCapsuleComponent)))) "100.000000,100.000000,100.000000" "0, 0, 0" (Utilities|Array|MakeArray "ObjectTypeQuery3") false _outactors "ForOneFrame" true))
  (if _returnvalue
    (Variables|Default|SetSP4HitLocation (Transformation|GetActorLocation (.HitActor (Collision|BreakHitResult _outhit))))
    (if (<= (.Distance (Collision|BreakHitResult _outhit)) 2e+02)
      (switch Utilities|FlowControl|Switch|SwitchonE_CharacterRotation (Variables|Default|GetCharacterRotation)
        (:NewEnumerator0
          (Pawn|SetControlRotation (Pawn|GetController) (Math|Rotator|MakeRotator 0.0 0.0 1.8e+02)))
        (:NewEnumerator1
          (Pawn|SetControlRotation (Pawn|GetController) (Math|Rotator|MakeRotator 0.0 0.0 0.0))))
      (Transformation|SetWorldLocation (Variables|Default|GetCapsuleComponent) (+ (Variables|Default|GetSP4HitLocation) (* (Variables|Default|GetSP4SmashLocationOffset) (Math|Vector|GetForwardVector (Variables|Default|GetCapsuleComponent)) "-1.000000,0.000000,0.000000")) false false)
      (else
        (Transformation|SetWorldLocation (Variables|Default|GetCapsuleComponent) (+ (Variables|Default|GetSP4HitLocation) (* (Variables|Default|GetSP4SmashLocationOffset) (Math|Vector|GetForwardVector (Variables|Default|GetCapsuleComponent)))) false false)))
    (Rendering|SetVisibility (Variables|Default|GetSprite) true false :!label _label)
    (Class|BPICombo|SP4SmashStart(Message) (Variables|/Script/PaperZD.PaperZDAnimationComponent|GetAnimInstance (Variables|Default|GetAnimationComponent)))
    (Variables|/Script/Engine.CharacterMovementComponent|SetGravityScale (Variables|Character|GetCharacterMovement) 3.0)
    (else
      (Components|Timeline|SetPlayRate (Variables|Default|GetSP4Dash) 16.0)
      (bind _sp4dash (Timeline|SP4Dash PlayFromStart)
        (:Update
          (Transformation|SetWorldLocation (Variables|Default|GetCapsuleComponent) (Math|Vector|Lerp(Vector) (Variables|Default|GetSP4StartLocation) (+ (Variables|Default|GetSP4StartLocation) (* (Variables|Default|GetSP4TraceDistance) (Math|Vector|GetForwardVector (Variables|Default|GetCapsuleComponent)))) _sp4dash) true false))
        (:Finished
          (goto _label))))))

(event Game|Damage|EventAnyDamage
  (params (Damage :type Float%20%28single-precision%29) (DamageType :type Damage%20Type%20Object%20Reference) (InstigatedBy :type Controller%20Object%20Reference) (DamageCauser :type Actor%20Object%20Reference))
  (if (Variables|Default|GetIsEvading)
    (CallFunction|AddCC 1)
    (else
      (|CallParentFunction Damage 0 0 0)
      (CallFunction|ResetComboHits)
      (Default|UpdateHP (Variables|Default|GetHUDReference) (Variables|Default|GetCurrentHP) (Variables|Default|GetMaxHP)))))

(event EventExcutedAnAttack
  (params (CCConsume :type Integer))
  (Variables|Default|SetCurrentChainCapacity (- (Variables|Default|GetCurrentChainCapacity) CCConsume))
  (CallFunction|SetHitEnemyasTarget)
  (CallFunction|SetTagHideforOthers)
  (Utilities|Array|Clear (Variables|Default|GetTargetHitThisAttack))
  (bind _returnvalue (Actor|GetActorOfClass "/Game/Blueprints/TestCamera.TestCamera_C"))
  (Class|BPITellCameratoDo|BlendScopeTarget(Message) _returnvalue)
  (Default|UpdateCurrentCC (Variables|Default|GetHUDReference)))

(event EventDeliverAttackParametertoAttacker
  (params (AttackParameter :type F%20Attacks%20Structure))
  (|CallParentFunction AttackParameter))

(fn ConstructionScript
  (|CallParentFunction))

(fn ResetAttackStage
  (if (Variables|Default|GetIsAttacking)
    (Variables|Default|SetAttackStage 0)))

(fn CanJumpCheck
  (bind _asabp_yusuke (Utilities|Casting|CastToABP_Yusuke (Variables|/Script/PaperZD.PaperZDAnimationComponent|GetAnimInstance (Variables|Default|GetAnimationComponent))))
  (if (or (not (GameplayTags|HasTag (Variables|/Game/Blueprints/Characters/Yusuke/ABP_Yusuke.ABP_Yusuke_C|GetComboAnimationTags _asabp_yusuke) "(TagName=\"Combo\")")) (GameplayTags|HasTag (Variables|/Game/Blueprints/Characters/Yusuke/ABP_Yusuke.ABP_Yusuke_C|GetComboAnimationTags _asabp_yusuke) "(TagName=\"Combo.CanCancel\")"))
    (return true)))

(fn SetAttackDirection
  (switch Utilities|FlowControl|Switch|SwitchonE_CharacterDirectionalInput (Variables|Default|GetDirectionalInput)
    (:NewEnumerator0
      _)
    (:NewEnumerator5
      _)
    (:NewEnumerator6
      _)
    (:NewEnumerator1
      (return "NewEnumerator4"))
    (:NewEnumerator7
      (return "NewEnumerator4"))
    (:NewEnumerator8
      (return "NewEnumerator4"))
    (:NewEnumerator2
      (switch Utilities|FlowControl|Switch|SwitchonE_CharacterRotation (Variables|Default|GetCharacterRotation)
        (:NewEnumerator0
          (return "NewEnumerator1"))
        (:NewEnumerator1
          (return "NewEnumerator2"))))
    (:NewEnumerator3
      (switch Utilities|FlowControl|Switch|SwitchonE_CharacterRotation (Variables|Default|GetCharacterRotation)
        (:NewEnumerator0
          (return "NewEnumerator2"))
        (:NewEnumerator1
          (return "NewEnumerator1"))))
    (:NewEnumerator4
      (return "NewEnumerator0")))
  (return "NewEnumerator3"))

(fn SetTagHideforOthers
  (CallFunction|GetAllEnemies)
  (Utilities|Array|RemoveItem (Variables|Default|GetAllEnemies) (Variables|Default|GetAttackTarget))
  (for _array_element (Variables|Default|GetAllEnemies)
    (Rendering|SetVisibility (Variables|/Game/Blueprints/Characters/BP_RPGChar.BP_RPGChar_C|GetTargetTagWidget _array_element) false false)))

(fn GetAllEnemies
  ;[1 1 1] On Battle start, get all the enemies
  (bind _outactors (Actor|GetAllActorsOfClass "/Game/Blueprints/Characters/BP_RPGChar.BP_RPGChar_C"))
  (for _array_element _outactors
    (if (!= (Variables|/Game/Blueprints/Characters/BP_RPGChar.BP_RPGChar_C|GetFaction _array_element) (Variables|Default|GetFaction))
      (Utilities|Array|Add (Variables|Default|GetAllEnemies) _array_element))))

(fn SetFirstTarget
  ;[1 1 1] On Battle start, choose the nearest enemy automatically
  (Variables|Default|SetCompareEnemy (Utilities|Array|Get(acopy) (Variables|Default|GetAllEnemies)))
  (for (_array_element _array_index) (Variables|Default|GetAllEnemies)
    (if (!= _array_index 0)
      (if (< (Transformation|GetDistanceTo _array_element self) (Transformation|GetDistanceTo (Variables|Default|GetCompareEnemy) self))
        (Variables|Default|SetCompareEnemy _array_element))))
  (bind _output_get (Variables|Default|SetAttackTarget (Variables|Default|GetCompareEnemy)))
  (Rendering|SetVisibility (Variables|/Game/Blueprints/Characters/BP_RPGChar.BP_RPGChar_C|GetTargetTagWidget _output_get) true false))

(fn SetHitEnemyasTarget
  (if (not (Utilities|Array|IsEmpty (Variables|Default|GetTargetHitThisAttack)))
    (if (== (Utilities|Array|FindItem (Variables|Default|GetTargetHitThisAttack) (Variables|Default|GetAttackTarget)) -1)
      (bind _output_get (Variables|Default|SetAttackTarget (Utilities|Array|Get(acopy) (Variables|Default|GetTargetHitThisAttack))))
      (Rendering|SetVisibility (Variables|/Game/Blueprints/Characters/BP_RPGChar.BP_RPGChar_C|GetTargetTagWidget _output_get) true false))))

(fn SenseDirectionalInput
  (bind _returnvalue (Input|EnhancedActionValues|GetIA_Move))
  (bind _x (Math|Vector2D|BreakVector2D _returnvalue))
  (Math|Float|CompareFloat (.Y (Math|Vector2D|BreakVector2D (Input|EnhancedActionValues|GetIA_Move))) 0.0
    (:>
      (Math|Float|CompareFloat (.X (Math|Vector2D|BreakVector2D (Input|EnhancedActionValues|GetIA_Move))) 0.0
        (:>
          (Variables|Default|SetDirectionalInput "NewEnumerator6"))
        (:==
          (Variables|Default|SetDirectionalInput "NewEnumerator0"))
        (:<
          (Variables|Default|SetDirectionalInput "NewEnumerator5"))))
    (:==
      (Math|Float|CompareFloat _x 0.0
        (:>
          (Variables|Default|SetDirectionalInput "NewEnumerator2"))
        (:==
          (Variables|Default|SetDirectionalInput "NewEnumerator4"))
        (:<
          (Variables|Default|SetDirectionalInput "NewEnumerator3"))))
    (:<
      (Math|Float|CompareFloat _x 0.0
        (:>
          (Variables|Default|SetDirectionalInput "NewEnumerator8"))
        (:==
          (Variables|Default|SetDirectionalInput "NewEnumerator1"))
        (:<
          (Variables|Default|SetDirectionalInput "NewEnumerator7"))))))

(fn SetEvadeVector
  (switch Utilities|FlowControl|Switch|SwitchonE_CharacterDirectionalInput (Variables|Default|GetDirectionalInput)
    (:NewEnumerator0
      (return (+ (Variables|AttackParameter|GetEvadeStartLocation) (* (Variables|AttackParameter|GetEvadeVector) "0.000000,-1.000000,1.000000"))))
    (:NewEnumerator5
      (return (+ (Variables|AttackParameter|GetEvadeStartLocation) (* (Variables|AttackParameter|GetEvadeVector) "-1.000000,-1.000000,1.000000"))))
    (:NewEnumerator6
      (return (+ (Variables|AttackParameter|GetEvadeStartLocation) (* (Variables|AttackParameter|GetEvadeVector) "1.000000,-1.000000,1.000000"))))
    (:NewEnumerator1
      (return (+ (Variables|AttackParameter|GetEvadeStartLocation) (* (Variables|AttackParameter|GetEvadeVector) "0.000000,1.000000,1.000000"))))
    (:NewEnumerator7
      (return (+ (Variables|AttackParameter|GetEvadeStartLocation) (* (Variables|AttackParameter|GetEvadeVector) "-1.000000,1.000000,1.000000"))))
    (:NewEnumerator8
      (return (+ (Variables|AttackParameter|GetEvadeStartLocation) (* (Variables|AttackParameter|GetEvadeVector) "1.000000,1.000000,1.000000"))))
    (:NewEnumerator2
      (return (+ (Variables|AttackParameter|GetEvadeStartLocation) (* (Variables|AttackParameter|GetEvadeVector) "1.000000,0.000000,1.000000"))))
    (:NewEnumerator3
      (return (+ (Variables|AttackParameter|GetEvadeStartLocation) (* (Variables|AttackParameter|GetEvadeVector) "-1.000000,-0.000000,1.000000"))))))

(fn AddCC
  (params (CCAdd :type Integer))
  (Variables|Default|SetCurrentChainCapacity (Math|Integer|Clamp(Integer) (+ (Variables|Default|GetCurrentChainCapacity) CCAdd) 0 (Variables|Default|GetMaxChainCapacity)))
  (Default|UpdateCurrentCC (Variables|Default|GetHUDReference)))