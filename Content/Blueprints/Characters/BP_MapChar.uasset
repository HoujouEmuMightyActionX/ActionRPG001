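; BP_MapChar is a map character that turns to face its horizontal direction of travel along the X axis.
; Every Tick, UpdateControllerRotation checks the sign of the movement component's X velocity and snaps the controller's yaw to face forward or backward, provided a controller is valid.
; At zero X velocity the rotation is left untouched, so the last facing persists.
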(event EventBeginPlay)

(event Collision|EventActorBeginOverlap
  (params (OtherActor :type Actor%20Object%20Reference)))

(event EventTick
  (params (DeltaSeconds :type Float%20%28single-precision%29))
  (CallFunction|UpdateControllerRotation))

(fn ConstructionScript)

(fn UpdateControllerRotation
  (bind _returnvalue (Pawn|GetController))
  (bind _returnvalue_2 (Pawn|GetController))
  (Math|Float|CompareFloat (.x (Variables|/Script/Engine.MovementComponent|GetVelocity (Variables|Character|GetCharacterMovement))) 0.0
    (:>
      (Utilities|IsValid _returnvalue
        (:Is%20Valid
          (Pawn|SetControlRotation _returnvalue (Math|Rotator|MakeRotator 0.0 0.0 0.0)))))
    (:<
      (Utilities|IsValid _returnvalue_2
        (:Is%20Valid
          (Pawn|SetControlRotation _returnvalue_2 (Math|Rotator|MakeRotator 0.0 0.0 1.8e+02)))))))