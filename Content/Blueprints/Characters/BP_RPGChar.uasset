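; Sprite-based RPG character with two-way facing, handling both sides of combat: dealing hits and reacting to them.
; Hitbox overlaps damage other factions, send attack parameters by interface, spawn hit marks and fill a critical gauge that boosts damage when full.
; Received hits flash a dynamic material, then launch, knock back, slam or stun with sprite shake.
; Damage states use retriggerable-delay polling for landing, and hit stop uses CustomTimeDilation.
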(event OnComponentBeginOverlap(Hitbox)
  (params (OverlappedComponent :type Primitive%20Component%20Object%20Reference) (OtherActor :type Actor%20Object%20Reference) (OtherComp :type Primitive%20Component%20Object%20Reference) (OtherBodyIndex :type Integer) (bFromSweep :type Boolean) (SweepResult :type Hit%20Result%20Structure%20%28by%20ref%29))
  (bind _hitbox (Variables|Default|GetHitbox))
  (bind _currentattackparameter (Variables|Default|GetCurrentAttackParameter))
  (bind _currentattackparameter_2 (Variables|Default|GetCurrentAttackParameter))
  (bind _basedamage (Utilities|Struct|BreakF_Attacks _currentattackparameter_2))
  (bind (_hitboxlocation _basedamage_2 _hitboxextent _attackeffect _launch_delay _launch_power _knockback_delay _knockback_power _slap_delay _slap_power) (Utilities|Struct|BreakF_Attacks _currentattackparameter))
  (bind _returnvalue (Transformation|GetWorldLocation _hitbox))
  (bind _asbp_rpgchar (Utilities|Casting|CastToBP_RPGChar OtherActor))
  (if (!= (Variables|BP_RPGChar_C|GetFaction _asbp_rpgchar) (Variables|Parameter|GetFaction))
    (if (== (Variables|Default|GetCriticalCage) 1.0)
      (Game|Damage|ApplyDamage _asbp_rpgchar (* _basedamage 1.5) (Pawn|GetController) self)
      (else
        (Game|Damage|ApplyDamage _asbp_rpgchar _basedamage (Pawn|GetController) self)))
    (if (not (Utilities|Enum|Equal(Enum) (Variables|BP_RPGChar_C|GetDamageState _asbp_rpgchar) "NewEnumerator2"))
      (Class|BPIActiontoCharacter|DeliverAttackParametertoTarget(Message) _asbp_rpgchar _attackeffect _launch_delay _launch_power _knockback_delay _knockback_power _slap_delay _slap_power self)
      (CallFunction|HitStopSequence 0.0 0.01)
      (bind _outhits (Class|KismetSystemLibrary|BoxTraceMultiforObjects _returnvalue _returnvalue (Variables|/Script/Engine.BoxComponent|GetBoxExtent (Variables|Default|GetHitbox)) "0, 0, 0" (Variables|Default|GetObject%20Types) false 0 "ForOneFrame" true))
      (for _array_element _outhits
        (if (Utilities|Enum|Equal(Enum) (Variables|CharacterState|GetCharacterRotation) "NewEnumerator0")
          (Game|SpawnActorfromClass (Variables|Default|GetHitMarkVFX) (Math|Transform|MakeTransform (+ (/ (- (.Location (Collision|BreakHitResult _array_element)) (Transformation|GetActorLocation (.HitActor (Collision|BreakHitResult _array_element)))) "2.000000,2.000000,2.000000") (Transformation|GetActorLocation (.HitActor (Collision|BreakHitResult _array_element)))) "1.000000,1.0,1.0" "1.000000,1.000000,1.000000") "AlwaysSpawn" "MultiplyWithRoot" 0 0)
          (else
            (Game|SpawnActorfromClass (Variables|Default|GetHitMarkVFX) (Math|Transform|MakeTransform (+ (+ (/ (- (.Location (Collision|BreakHitResult _array_element)) (Transformation|GetActorLocation (.HitActor (Collision|BreakHitResult _array_element)))) "2.000000,2.000000,2.000000") (Transformation|GetActorLocation (.HitActor (Collision|BreakHitResult _array_element)))) "0.000000,20.000000,0.000000") "1.000000,180.0,1.0" "1.000000,1.000000,1.000000") "AlwaysSpawn" "MultiplyWithRoot" 0 0)))
        (if (== (Variables|Default|GetCriticalCage) 1.0)
          (Variables|Default|SetCriticalCage 0.0)
          (else
            (Variables|Default|SetCriticalCage (+ (.CriticalCageIncrease (Utilities|Struct|BreakF_Attacks (Variables|Default|GetCurrentAttackParameter))) (Variables|Default|GetCriticalCage)))))))))

(event Custom|HitStopSequence
  (params (HitStopStartDelay :type Float%20%28single-precision%29) (HitStoplength :type Float%20%28single-precision%29))
  ;[1 1 1] 受击，仅处理伤害不处理表现
  (Utilities|FlowControl|RetriggerableDelay HitStopStartDelay)
  (Variables|Default|SetCustomTimeDilation 0.0)
  (Utilities|FlowControl|RetriggerableDelay HitStoplength)
  (Variables|Default|SetCustomTimeDilation 1.0))

(event Custom|SpriteShake
  (bind _spritebaselocation (Variables|Reference|GetSpriteBaseLocation))
  ;[1 1 1] 受击，仅处理伤害不处理表现
  (bind _isa (Utilities|FlowControl|FlipFlop)
    (:A
      _)
    (:B
      _))
  (Transformation|SetRelativeLocation (Variables|Default|GetSprite) (Math|Vector|MakeVector (+ (.x _spritebaselocation) (Math|Float|SelectFloat (* (Variables|GameFeel|GetSpriteShakeDistance) -1.0) (Variables|GameFeel|GetSpriteShakeDistance) _isa)) (.y _spritebaselocation) (.z _spritebaselocation)) false false))

(event Custom|Float
  (Variables|Default|SetDamageState "NewEnumerator1")
  (Utilities|FlowControl|RetriggerableDelay 0.1)
  (if (AI|Components|NavMovement|IsMovingonGround (Variables|Character|GetCharacterMovement)) :!label _label
    (Utilities|Time|ClearandInvalidateTimerbyHandle (Variables|Reference|GetSpriteShakeHandle))
    (Variables|Default|SetDamageState "NewEnumerator2")
    (Utilities|FlowControl|RetriggerableDelay 2.0)
    (CallFunction|LeaveDamagedState)
    (else
      (Utilities|FlowControl|RetriggerableDelay 0.02)
      (goto _label))))

(event Custom|Stun
  (Variables|Default|SetDamageState "NewEnumerator0")
  (bind _returnvalue (Utilities|Time|SetTimerbyEvent (EventDispatchers|CreateEvent :!event Custom|SpriteShake) 0.02 true 0.02))
  (Variables|Reference|SetSpriteShakeHandle _returnvalue)
  (CallFunction|HitStopSequence 0.0 0.2)
  (Utilities|FlowControl|RetriggerableDelay 0.6)
  (if (Utilities|Enum|Equal(Enum) (Variables|Default|GetDamageState) "NewEnumerator0")
    (Utilities|Time|ClearandInvalidateTimerbyHandle (Variables|Reference|GetSpriteShakeHandle))
    (CallFunction|LeaveDamagedState)))

(event Custom|HitFlash
  (params (FlashStrength :type Float%20%28single-precision%29) (FlashColor :type Linear%20Color%20Structure) (FadeSpeed :type Float%20%28single-precision%29))
  ;[1 1 1] 受击，仅处理伤害不处理表现
  (Rendering|Material|SetScalarParameterValue (Variables|Default|GetDynamicSpriteMat) "FlashMultiplier" FlashStrength :!class /Script/Engine.MaterialInstanceDynamic)
  (Rendering|Material|SetVectorParameterValue (Variables|Default|GetDynamicSpriteMat) "FlashColor" FlashColor :!class /Script/Engine.MaterialInstanceDynamic)
  (Components|Timeline|SetPlayRate (Variables|Default|GetFlashFadeOut) FadeSpeed)
  (bind _flashfadeout (Timeline|FlashFadeOut PlayFromStart)
    (:Update
      (Rendering|Material|SetScalarParameterValue (Variables|Default|GetDynamicSpriteMat) "FlashMultiplier" _flashfadeout :!class /Script/Engine.MaterialInstanceDynamic))))

(event EventBeginPlay
  (Variables|Reference|SetSpriteBaseLocation (Variables|/Script/Engine.SceneComponent|GetRelativeLocation (Variables|Default|GetSprite)))
  (Variables|Parameter|SetCurrentHP (Variables|Parameter|GetMaxHP))
  (Collision|SetCollisionEnabled (Variables|Default|GetHitbox) "NoCollision")
  (bind _returnvalue (Rendering|Material|CreateDynamicMaterialInstance (Variables|Default|GetSprite) 0 0 "None" :!class /Script/Engine.PrimitiveComponent))
  (Variables|Default|SetDynamicSpriteMat _returnvalue))

(event Collision|EventActorBeginOverlap
  (params (OtherActor :type Actor%20Object%20Reference)))

(event EventLeaveDamagedState
  (Variables|Default|SetDamageState "NewEnumerator3")
  (Default|CallDamagedStateSwitch false)
  (Variables|/Script/Engine.CharacterMovementComponent|SetGravityScale (Variables|Character|GetCharacterMovement) 3.0))

(event EventDeliverAttackParametertoTarget
  (params (AttackEffect :type E_AttackEffect%20Enum :default "NewEnumerator0") (LaunchDelay :type Float%20%28double-precision%29) (LaunchPower :type Vector :default "0, 0, 0") (KnockbackDelay :type Float%20%28double-precision%29) (KnockbackPower :type Vector :default "0, 0, 0") (SlapDelay :type Float%20%28double-precision%29) (SlapPower :type Vector :default "0, 0, 0") (Attacker :type BP%20RPG%20Char%20Object%20Reference))
  (switch Utilities|FlowControl|Switch|SwitchonE_AttackEffect (Utilities|Enum|ByteToEnumE_AttackEffect AttackEffect)
    (:NewEnumerator0
      (Utilities|FlowControl|RetriggerableDelay LaunchDelay)
      (Character|LaunchCharacter LaunchPower true true)
      (CallFunction|Float))
    (:NewEnumerator1
      (if (== (.Yaw (Math|Rotator|BreakRotator (Transformation|GetActorRotation Attacker))) 0.0)
        (Character|LaunchCharacter KnockbackPower true true)
        (CallFunction|Float)
        (else
          (Character|LaunchCharacter (* KnockbackPower "-1.000000,1.000000,1.000000") true false)
          (CallFunction|Float))))
    (:NewEnumerator3
      (Character|LaunchCharacter (* SlapPower "0.000000,0.000000,-1.000000") false true)
      (if (AI|Components|NavMovement|IsMovingonGround (Variables|Character|GetCharacterMovement)) :!label _label
        (Character|LaunchCharacter SlapPower false false)
        (CallFunction|Float)
        (else
          (Utilities|FlowControl|RetriggerableDelay 0.02)
          (goto _label))))
    (:NewEnumerator4
      (Character|LaunchCharacter "0.000000,0.000000,200.000000" true true)
      (CallFunction|Stun))))

(event EventTick
  (params (DeltaSeconds :type Float%20%28single-precision%29))
  (if (== (.yaw (Pawn|GetControlRotation :!class /Script/Engine.Pawn)) 1.8e+02)
    (Variables|CharacterState|SetCharacterRotation "NewEnumerator1")
    (else
      (Variables|CharacterState|SetCharacterRotation "NewEnumerator0"))))

(event Game|Damage|EventAnyDamage
  (params (Damage :type Float%20%28single-precision%29) (DamageType :type Damage%20Type%20Object%20Reference) (InstigatedBy :type Controller%20Object%20Reference) (DamageCauser :type Actor%20Object%20Reference))
  ;[1 1 1] 受击，仅处理伤害不处理表现
  (CallFunction|ReceiveAttack Damage)
  (if (<= (Variables|Parameter|GetCurrentHP) 0.0)
    (Variables|Default|SetDamageState "NewEnumerator4")
    (Utilities|FlowControl|Delay 0.6)
    (Actor|DestroyActor)))

(event EventDeliverAttackParametertoAttacker
  (params (AttackParameter :type F%20Attacks%20Structure))
  (Variables|Default|SetCurrentAttackParameter AttackParameter)
  (Math|Float|CompareFloat (Variables|Default|GetCriticalCage) 1.0
    (:==
      (Variables|Default|SetHitMarkVFX "/Game/VFX/BP_HitMarkHeavy.BP_HitMarkHeavy_C"))
    (:<
      (Variables|Default|SetHitMarkVFX "/Game/VFX/BP_HitMarkLight.BP_HitMarkLight_C"))))

(fn ConstructionScript)

(fn UpdateControllerRotation
  (bind _returnvalue (Pawn|GetController))
  (bind _returnvalue_2 (Pawn|GetController))
  (Math|Float|CompareFloat (.x (Variables|/Script/Engine.MovementComponent|GetVelocity (Variables|Character|GetCharacterMovement))) 0.0
    (:>
      (Utilities|IsValid _returnvalue
        (:Is%20Valid
          (Pawn|SetControlRotation _returnvalue (Math|Rotator|MakeRotator 0.0 0.0 0.0)))))
    (:<
      (Utilities|IsValid _returnvalue_2
        (:Is%20Valid
          (Pawn|SetControlRotation _returnvalue_2 (Math|Rotator|MakeRotator 0.0 0.0 1.8e+02)))))))

(fn ReceiveAttack
  (params (ReceivedDamage :type Float%20%28double-precision%29))
  (Development|PrintString (Utilities|String|ToString(Float) ReceivedDamage))
  (Variables|Parameter|SetCurrentHP (- (Variables|Parameter|GetCurrentHP) ReceivedDamage))
  (Audio|PlaySoundatLocation "/Game/Sound/Hit/Cue_Hit.Cue_Hit" "0, 0, 0" "0, 0, 0" 1.0 1.0 0.0 0 0 0 0)
  (Class|PaperZDAnimInstance|StopAllAnimationOverrides (Variables|/Script/PaperZD.PaperZDAnimationComponent|GetAnimInstance (Variables|Default|GetAnimationComponent)))
  (CallFunction|HitFlash 1e+01 "(R=0.962442,G=0.978911,B=1.000000,A=1.000000)" 2e+01)
  (Default|CallDamagedStateSwitch true))

(fn CanActCheck
  (return (and (not (Variables|CharacterState|GetIsAttacking)) (Utilities|Enum|Equal(Enum) (Variables|Default|GetDamageState) "NewEnumerator3"))))